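; BP_DoorBegin is a door Blueprint that raises a Cube when one trigger box is overlapped and resets it when a second is overlapped.
; Box stores the Cube's position and plays a Timeline that lerps it to a fixed world height.
; Box1 snaps the Cube back to the stored position without stopping the Timeline.
; An Enter flag makes the two triggers alternate.
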(event `self.Box.OnComponentBeginOverlap`
  (params (OverlappedComponent :type "PrimitiveComponent Object Reference") (OtherActor :type "Actor Object Reference") (OtherComp :type "PrimitiveComponent Object Reference") (OtherBodyIndex :type Integer) (bFromSweep :type Boolean) (SweepResult :type "HitResult Structure (by ref)"))
  (bind _basepos (`self.basePos`))
  (if (not (`self._enter`))
    (set `self._enter` true)
    (set `self.basePos` (`SceneComponent.K2_GetComponentLocation` (`self.Cube`)))
    (bind (_direction _aplha) (`Timeline|Timeline` :!via `PlayFromStart`)
      (:`Update`
        (`SceneComponent.K2_SetWorldLocation` (`self.Cube`) (`KismetMathLibrary.VLerp` _basepos (`KismetMathLibrary.MakeVector` (.x _basepos) (.y _basepos) 1000.0) _aplha) false false)))))

(event `self.Box1.OnComponentBeginOverlap`
  (params (OverlappedComponent :type "PrimitiveComponent Object Reference") (OtherActor :type "Actor Object Reference") (OtherComp :type "PrimitiveComponent Object Reference") (OtherBodyIndex :type Integer) (bFromSweep :type Boolean) (SweepResult :type "HitResult Structure (by ref)"))
  (if (`self._enter`)
    (set `self._enter` false)
    (`SceneComponent.K2_SetWorldLocation` (`self.Cube`) (`self.basePos`) false false)))

(fn `UserConstructionScript`)