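; BP_Door is an interactable door that opens only when its Key reference is invalid, then destroys itself.
; On Interact it clears RenderDoor on the EuclidianToDeactivate entries and sets it on the EuclidianToActivate entries, switching which linked Euclidian doors render.
; Only the activation loop checks validity, as the deactivation loop's IsValid check is disconnected.
; GetInteractiveState always returns one fixed enum value.
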(event `/Game/FirstPerson/Blueprints/BP_Game/BPI_Interation.Interact`
  (`/Engine/EditorBlueprintResources/StandardMacros.IsValid` (`self._key`)
    (:`Is Not Valid`
      (for _array_element (`self.euclidianToDeactivate`)
        (set `/Game/EuclidianDoor._renderDoor` false _array_element))
      (for _array_element_2 (`self.euclidianToActivate`)
        (`/Engine/EditorBlueprintResources/StandardMacros.IsValid` _array_element_2
          (:`Is Valid`
            (set `/Game/EuclidianDoor._renderDoor` true _array_element_2))))
      (`self.K2_DestroyActor`))))

(fn `GetInteractiveState`
  (returns (state :type "/Game/FirstPerson/Blueprints/Enum/E_SelectInterface Enum"))
  (return "NewEnumerator1"))

(fn `UserConstructionScript`)