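; Lockable non-Euclidean portal door that shows the view through its linked portal and teleports the player seamlessly across.
; While unlocked and rendering, Tick recursively captures the linked camera, deepest first, into a viewport-sized render target on PortalPlane, using clip planes.
; Camera crossings of the door plane remap player transform, control rotation and velocity to the linked portal.
; Interact unlocks it once the Key actor is invalid, removing the HUD key.
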(event `self.ReceiveBeginPlay`
  (bind (_returnvalue_x _returnvalue_y) (`KismetMathLibrary.BreakVector2D` (`WidgetLayoutLibrary.GetViewportSize`)))
  (bind _asbp_first_person_character (cast `/Game/FirstPerson/Blueprints/BP_FirstPersonCharacter` (`GameplayStatics.GetPlayerCharacter` 0)))
  (set `self.WBP Key` (`/Game/FirstPerson/Blueprints/BP_FirstPersonCharacter.WBP_Key` _asbp_first_person_character))
  (`self.SetTickGroup` "TG_PostUpdateWork")
  (bind _returnvalue (`KismetMaterialLibrary.CreateDynamicMaterialInstance` "/Game/euclidianTest/Door/Mat_PortalMaterial.Mat_PortalMaterial"))
  (bind _output_get (set `self._portalMat` _returnvalue))
  (`PrimitiveComponent.SetMaterial` (`self.PortalPlane`) 0 _output_get)
  (bind _returnvalue_2 (`KismetRenderingLibrary.CreateRenderTarget2D` (`KismetMathLibrary.FTrunc` _returnvalue_x) (`KismetMathLibrary.FTrunc` _returnvalue_y)))
  (bind _output_get_2 (set `self._portalRT` _returnvalue_2))
  (`MaterialInstanceDynamic.SetTextureParameterValue` (`self._portalMat`) "PortalTexture" _output_get_2)
  (`self.CE_SetTextureTarget` :!label _label)
  (`self.SetClipPlanes`)
  (`MaterialInstanceDynamic.SetVectorParameterValue` (`self._portalMat`) "OffsetDistance" (`KismetMathLibrary.MakeColor` (.x (* (`SceneComponent.GetForwardVector` (`self.Arrow`)) (`self.OffsetAmount`))) (.y (* (`SceneComponent.GetForwardVector` (`self.Arrow`)) (`self.OffsetAmount`))) (.z (* (`SceneComponent.GetForwardVector` (`self.Arrow`)) (`self.OffsetAmount`)))))
  (set `self._renderDoor` (`self._IsRenderingFromStart`))
  (if (not (`self._IsLocked`))
    (`self.CE_UnlockDoor`)))

(event `CE_OnLateSet`
  (goto _label))

(event `CE_SetTextureTarget`
  (bind __linkedportal (`self._linkedPortal`))
  (`/Engine/EditorBlueprintResources/StandardMacros.IsValid` __linkedportal
    (:`Is Valid`
      (set `SceneCaptureComponent2D.TextureTarget` (`self._portalRT`) (`/Game/BP_EuclidianDoorSuspended.PortalCamera` __linkedportal)))))

(event `self.ReceiveTick`
  (params (DeltaSeconds :type "Float (single-precision)"))
  (if (`self._IsLocked`)
    _
    (elif (`self._renderDoor`)
      (`self.UpdateSceneCaptureRecursive` (0.0 0.0 0.0))
      (`self.CheckWiewportSize`)
      (`self.CheckTeleport`))))

(event `CE_SetRender`
  (params (value :type Boolean))
  (set `self._renderDoor` value))

(event `CE_SetUnlock`
  (params (state :type Boolean))
  (set `self._IsLocked` state))

(event `self.Interact`
  (if (`self._IsLocked`)
    (`/Engine/EditorBlueprintResources/StandardMacros.IsValid` (`self._key`)
      (:`Is Not Valid`
        (`self.CE_UnlockDoor`)
        (`/Game/FirstPerson/UI/WBP_Key.CE_RemouvKey` (`self.WBP Key`))
        (`AudioComponent.Play` (`self.Unlok`) 0.0)))))

(event `CE_UnlockDoor`
  (set `self._IsLocked` false)
  (set `self.interactiveState` "NewEnumerator7")
  (`PrimitiveComponent.SetCollisionEnabled` (`self.PortalPlane`) "NoCollision"))

(fn `CheckTeleport`
  (`/Engine/EditorBlueprintResources/StandardMacros.IsValid` (`|GetArrayItem` (`PrimitiveComponent.GetOverlappingActors` (`self.Box`) "/Game/FirstPerson/Blueprints/BP_FirstPersonCharacter.BP_FirstPersonCharacter_C"))
    (:`Is Valid`
      (bind _out (`self.IsPointCrossingPortals` (`SceneComponent.K2_GetComponentLocation` (`/Game/FirstPerson/Blueprints/BP_FirstPersonCharacter.FirstPersonCamera` (cast `/Game/FirstPerson/Blueprints/BP_FirstPersonCharacter` (`GameplayStatics.GetPlayerCharacter` 0) :!pure true))) (`self.K2_GetActorLocation`) (`KismetMathLibrary.NegateVector` (`SceneComponent.GetForwardVector` (`self.Arrow`)))))
      (if _out
        (`self.TeleportCharacter`)))))

(fn `CheckWiewportSize`
  (bind (_returnvalue_x _returnvalue_y) (`KismetMathLibrary.BreakVector2D` (`WidgetLayoutLibrary.GetViewportSize`)))
  (bind __portalrt (`self._portalRT`))
  (bind (_x _y) (`KismetMathLibrary.BreakVector2D` (`WidgetLayoutLibrary.GetViewportSize`)))
  (if (not (and (== _x (`TextureRenderTarget2D.SizeX` __portalrt)) (== (`TextureRenderTarget2D.SizeY` __portalrt) _y)))
    (`KismetSystemLibrary.PrintString` "RESIZING")
    (`KismetRenderingLibrary.ResizeRenderTarget2D` (`self._portalRT`) (`KismetMathLibrary.FTrunc` _returnvalue_x) (`KismetMathLibrary.FTrunc` _returnvalue_y))))

(fn `GetInteractiveState`
  (returns (state :type "/Game/FirstPerson/Blueprints/Enum/E_SelectInterface Enum"))
  (bind _interactivestate (`self.interactiveState`))
  (`KismetSystemLibrary.PrintString` (`|GetEnumeratorNameAsString` _interactivestate))
  (return _interactivestate))

(fn `IsPointCrossingPortals`
  (params (Point :type "Vector Structure") (PortalLocation :type "Vector Structure") (PortalNormal :type "Vector Structure"))
  (returns (out :type Boolean))
  (locals (PortalPlane :type "Plane Structure") (IsIntersect :type Boolean) (IsInFront :type Boolean) (IsCrossing :type Boolean))
  (set `self.LastInFront` (>= (`KismetMathLibrary.Dot_VectorVector` PortalNormal (- Point PortalLocation)) 0.0))
  (bind _output_get (set `local.PortalPlane` (`KismetMathLibrary.MakePlaneFromPointAndNormal` (`local.PortalLocation`) (`local.PortalNormal`))))
  (set `local.IsIntersect` (`.ReturnValue` (`KismetMathLibrary.LinePlaneIntersection` (`self.LastPosition`) (`local.Point`) _output_get)))
  (set `local.IsCrossing` (and (`local.IsIntersect`) (not (`local.IsInFront`)) (`self.LastInFront`)))
  (set `self.LastInFront` (`local.IsInFront`))
  (set `self.LastPosition` (`local.Point`))
  (return (`local.IsCrossing`)))

(fn `SetClipPlanes`
  (bind __linkedportal (`self._linkedPortal`))
  (`/Engine/EditorBlueprintResources/StandardMacros.IsValid` __linkedportal
    (:`Is Valid`
      (`/Engine/EditorBlueprintResources/StandardMacros.IsValid` (`/Game/BP_EuclidianDoorSuspended.PortalCamera` __linkedportal)
        (:`Is Valid`
          (set `SceneCaptureComponent2D.bEnableClipPlane` true (`self.PortalCamera`))
          (set `SceneCaptureComponent2D.ClipPlaneBase` (+ (`SceneComponent.K2_GetComponentLocation` (`self.PortalCamera`)) (* (`SceneComponent.GetForwardVector` (`self.Arrow`)) -30.0)) (`self.PortalCamera`))
          (set `SceneCaptureComponent2D.ClipPlaneNormal` (`SceneComponent.GetForwardVector` (`self.Arrow`)) (`self.PortalCamera`))
          (`KismetSystemLibrary.PrintString` "Hello"))))))

(fn `TeleportCharacter`
  (bind _returnvalue (`self.GetTransform`))
  (bind (_returnvalue_location _returnvalue_rotation _returnvalue_scale) (`KismetMathLibrary.BreakTransform` (`self.GetTransform`)))
  (bind _returnvalue_2 (`self.GetTransform`))
  (bind _returnvalue_3 (`Pawn.GetMovementComponent` (`GameplayStatics.GetPlayerCharacter` 0)))
  (bind (_x _y _z) (`KismetMathLibrary.GetAxes` (`Controller.GetControlRotation` (`GameplayStatics.GetPlayerController` 0))))
  (bind (_x_2 _y_2 _z_2) (`KismetMathLibrary.GetAxes` (`self.K2_GetActorRotation` (`GameplayStatics.GetPlayerCharacter` 0))))
  (bind _returnvalue_4 (`KismetMathLibrary.MakeRotationFromAxes` (`KismetMathLibrary.TransformDirection` (`self.GetTransform` (`self._linkedPortal`)) (`KismetMathLibrary.MirrorVectorByNormal` (`KismetMathLibrary.MirrorVectorByNormal` (`KismetMathLibrary.InverseTransformDirection` _returnvalue _x) (1.0 0.0 0.0)) (0.0 1.0 0.0))) (`KismetMathLibrary.TransformDirection` (`self.GetTransform` (`self._linkedPortal`)) (`KismetMathLibrary.MirrorVectorByNormal` (`KismetMathLibrary.MirrorVectorByNormal` (`KismetMathLibrary.InverseTransformDirection` _returnvalue _y) (1.0 0.0 0.0)) (0.0 1.0 0.0))) (`KismetMathLibrary.TransformDirection` (`self.GetTransform` (`self._linkedPortal`)) (`KismetMathLibrary.MirrorVectorByNormal` (`KismetMathLibrary.MirrorVectorByNormal` (`KismetMathLibrary.InverseTransformDirection` _returnvalue _z) (1.0 0.0 0.0)) (0.0 1.0 0.0)))))
  (`KismetSystemLibrary.PrintString` "TELEPORT")
  (`self.K2_SetActorLocationAndRotation` (`Controller.K2_GetPawn` (`GameplayStatics.GetPlayerController` 0)) (`KismetMathLibrary.TransformLocation` (`self.GetTransform` (`self._linkedPortal`)) (`KismetMathLibrary.InverseTransformLocation` (`KismetMathLibrary.MakeTransform` _returnvalue_location _returnvalue_rotation (`KismetMathLibrary.MakeVector` (* (.x _returnvalue_scale) -1.0) (* (.y _returnvalue_scale) -1.0) (.z _returnvalue_scale))) (`self.K2_GetActorLocation` (`GameplayStatics.GetPlayerCharacter` 0)))) (`KismetMathLibrary.MakeRotationFromAxes` (`KismetMathLibrary.TransformDirection` (`self.GetTransform` (`self._linkedPortal`)) (`KismetMathLibrary.MirrorVectorByNormal` (`KismetMathLibrary.MirrorVectorByNormal` (`KismetMathLibrary.InverseTransformDirection` _returnvalue_2 _x_2) (1.0 0.0 0.0)) (0.0 1.0 0.0))) (`KismetMathLibrary.TransformDirection` (`self.GetTransform` (`self._linkedPortal`)) (`KismetMathLibrary.MirrorVectorByNormal` (`KismetMathLibrary.MirrorVectorByNormal` (`KismetMathLibrary.InverseTransformDirection` _returnvalue_2 _y_2) (1.0 0.0 0.0)) (0.0 1.0 0.0))) (`KismetMathLibrary.TransformDirection` (`self.GetTransform` (`self._linkedPortal`)) (`KismetMathLibrary.MirrorVectorByNormal` (`KismetMathLibrary.MirrorVectorByNormal` (`KismetMathLibrary.InverseTransformDirection` _returnvalue_2 _z_2) (1.0 0.0 0.0)) (0.0 1.0 0.0)))) false false)
  (`Controller.SetControlRotation` (`GameplayStatics.GetPlayerController` 0) _returnvalue_4)
  (bind _vout (`self.UpdateVelocity` (`MovementComponent.Velocity` _returnvalue_3)))
  (set `MovementComponent.Velocity` _vout _returnvalue_3)
  (if (`self._rotatePlayer`)
    (`/Game/FirstPerson/Blueprints/BP_FirstPersonCharacter.CE_SmoothOrientation` (cast `/Game/FirstPerson/Blueprints/BP_FirstPersonCharacter` (`GameplayStatics.GetPlayerCharacter` 0) :!pure true) _returnvalue_4)))

(fn `Update Camera`
  (`SceneComponent.K2_SetWorldLocationAndRotation` (`/Game/BP_EuclidianDoorSuspended.PortalCamera` (`self._linkedPortal`)) (`self.Update Location` (0.0 0.0 0.0)) (`self.UpdateRotation` (struct)) false false))

(fn `Update Location`
  (params (OldLocation :type "Vector Structure"))
  (returns (ReturnValue :type "Vector Structure"))
  (return (`KismetMathLibrary.TransformLocation` (`self.GetTransform` (`self._linkedPortal`)) (`KismetMathLibrary.InverseTransformLocation` (`KismetMathLibrary.MakeTransform` (.location (`self.GetTransform`)) (.rotation (`self.GetTransform`)) (`KismetMathLibrary.MakeVector` (* (.x (.scale (`self.GetTransform`))) -1.0) (* (.y (.scale (`self.GetTransform`))) -1.0) (.z (.scale (`self.GetTransform`))))) OldLocation))))

(fn `UpdateRotation`
  (params (OldRotation :type "Rotator Structure"))
  (returns (ReturnValue :type "Rotator Structure"))
  (bind _returnvalue (`self.GetTransform`))
  (bind (_x _y _z) (`KismetMathLibrary.BreakRotIntoAxes` OldRotation))
  (bind _returnvalue_2 (`self.GetTransform` (`self._linkedPortal`)))
  (return (`KismetMathLibrary.MakeRotationFromAxes` (`KismetMathLibrary.TransformDirection` _returnvalue_2 (`KismetMathLibrary.MirrorVectorByNormal` (`KismetMathLibrary.MirrorVectorByNormal` (`KismetMathLibrary.InverseTransformDirection` _returnvalue _x) (1.0 0.0 0.0)) (0.0 1.0 0.0))) (`KismetMathLibrary.TransformDirection` _returnvalue_2 (`KismetMathLibrary.MirrorVectorByNormal` (`KismetMathLibrary.MirrorVectorByNormal` (`KismetMathLibrary.InverseTransformDirection` _returnvalue _y) (1.0 0.0 0.0)) (0.0 1.0 0.0))) (`KismetMathLibrary.TransformDirection` _returnvalue_2 (`KismetMathLibrary.MirrorVectorByNormal` (`KismetMathLibrary.MirrorVectorByNormal` (`KismetMathLibrary.InverseTransformDirection` _returnvalue _z) (1.0 0.0 0.0)) (0.0 1.0 0.0))))))

(fn `UpdateSceneCaptureRecursive`
  (params (Location :type "Vector Structure") (Rotation :type "Rotator Structure"))
  (locals (TemporaryLocation :type "Vector Structure" :default (0.0 0.0 0.0)) (TemporaryRotation :type "Rotator Structure"))
  (bind _temporarylocation (`local.TemporaryLocation`))
  (bind _temporaryrotation (`local.TemporaryRotation`))
  (bind _temporarylocation_2 (`local.TemporaryLocation`))
  (bind _temporaryrotation_2 (`local.TemporaryRotation`))
  (bind _transformcomponent (`PlayerCameraManager.TransformComponent` (`GameplayStatics.GetPlayerCameraManager` 0)))
  (bind _portalcamera (`/Game/BP_EuclidianDoorSuspended.PortalCamera` (`self._linkedPortal`)))
  (bind _portalcamera_2 (`/Game/BP_EuclidianDoorSuspended.PortalCamera` (`self._linkedPortal`)))
  (bind _portalcamera_3 (`/Game/BP_EuclidianDoorSuspended.PortalCamera` (`self._linkedPortal`)))
  (if (== (`self.CurrentRecursions`) 0)
    (set `local.TemporaryLocation` (`self.Update Location` (`SceneComponent.K2_GetComponentLocation` _transformcomponent)))
    (set `local.TemporaryRotation` (`self.UpdateRotation` (`SceneComponent.K2_GetComponentRotation` _transformcomponent)))
    (`/Engine/EditorBlueprintResources/StandardMacros.IncrementInt` (`self.CurrentRecursions`)
      (:`  `
        (`self.UpdateSceneCaptureRecursive` _temporarylocation_2 _temporaryrotation_2)
        (`SceneComponent.K2_SetWorldLocationAndRotation` _portalcamera _temporarylocation_2 _temporaryrotation_2 false false)
        (`SceneCaptureComponent2D.CaptureScene` _portalcamera)
        (set `self.CurrentRecursions` 0)))
    (elif (< (`self.CurrentRecursions`) (`self.MaxRecursions`))
      (set `local.TemporaryLocation` (`self.Update Location` (`local.Location`)))
      (set `local.TemporaryRotation` (`self.UpdateRotation` (`local.Rotation`)))
      (`/Engine/EditorBlueprintResources/StandardMacros.IncrementInt` (`self.CurrentRecursions`)
        (:`  `
          (`self.UpdateSceneCaptureRecursive` _temporarylocation _temporaryrotation)
          (`SceneComponent.K2_SetWorldLocationAndRotation` _portalcamera_2 _temporarylocation _temporaryrotation false false)
          (`SceneCaptureComponent2D.CaptureScene` _portalcamera_2)))
      (else
        (`SceneComponent.K2_SetWorldLocationAndRotation` _portalcamera_3 (`self.Update Location` (`local.Location`)) (`self.UpdateRotation` (`local.Rotation`)) false false)
        (`SceneComponent.SetVisibility` (`self.PortalPlane`) false false)
        (`SceneCaptureComponent2D.CaptureScene` _portalcamera_3)
        (`SceneComponent.SetVisibility` (`self.PortalPlane`) true false)))))

(fn `UpdateVelocity`
  (params (VelocityPlayer :type "Vector Structure"))
  (returns (VOut :type "Vector Structure"))
  (return (* (`KismetMathLibrary.TransformDirection` (`self.GetTransform` (`self._linkedPortal`)) (`KismetMathLibrary.MirrorVectorByNormal` (`KismetMathLibrary.MirrorVectorByNormal` (`KismetMathLibrary.InverseTransformDirection` (`self.GetTransform`) (`KismetMathLibrary.Normal` VelocityPlayer)) (1.0 0.0 0.0)) (0.0 1.0 0.0))) (`KismetMathLibrary.VSize` (`local.VelocityPlayer`)))))

(fn `UserConstructionScript`)