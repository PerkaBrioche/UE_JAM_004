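; A 3D main-menu button that, depending on its EButton type, either quits the game or opens Level_Euclidian1 with game-only input.
; BeginPlay sets the label text and font and caches the panel's base and slightly enlarged scales.
; Hover and UnHover drive two opposing timelines that stop each other and lerp from the current scale.
; Interact fires the action once, guarded by a Clicked flag, and GetInteractiveState returns a fixed enum value.
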(event `self.ReceiveBeginPlay`
  (bind _textrender (`self.TextRender`))
  (bind _output_get (set `self._BaseScale` (`SceneComponent.K2_GetComponentScale` (`self.Mesh_Panel`))))
  (set `self._targetScale` (* _output_get 1.02))
  (`TextRenderComponent.K2_SetText` _textrender (`self.Text`))
  (`TextRenderComponent.SetFont` _textrender "/Engine/EngineFonts/RobotoDistanceField.RobotoDistanceField"))

(event `/Game/FirstPerson/Blueprints/BP_Game/BPI_Interation.Hover`
  (`self.CE_Grow`))

(event `/Game/FirstPerson/Blueprints/BP_Game/BPI_Interation.UnHover`
  (`self.CE_UnGrow`))

(event `CE_StopGrow`
  (bind (_direction _alpha) (`Timeline|Timeline` :!via `Stop` :!label _label)
    (:`Update`
      (`SceneComponent.SetWorldScale3D` (`self.Mesh_Panel`) (`KismetMathLibrary.VLerp` (`self._actualScale`) (`self._targetScale`) _alpha)))))

(event `CE_Grow`
  (`self.CE_StopUnGrow`)
  (set `self._actualScale` (`SceneComponent.K2_GetComponentScale` (`self.Mesh_Panel`)))
  (goto _label :!via `PlayFromStart`))

(event `CE_StopUnGrow`
  (bind (_direction _alpha) (`Timeline|Timeline_0` :!via `Stop` :!label _label_2)
    (:`Update`
      (`SceneComponent.SetWorldScale3D` (`self.Mesh_Panel`) (`KismetMathLibrary.VLerp` (`self._actualScale`) (`self._BaseScale`) _alpha)))))

(event `CE_UnGrow`
  (`self.CE_StopGrow`)
  (set `self._actualScale` (`SceneComponent.K2_GetComponentScale` (`self.Mesh_Panel`)))
  (goto _label_2 :!via `PlayFromStart`))

(event `/Game/FirstPerson/Blueprints/BP_Game/BPI_Interation.Interact`
  (bind _returnvalue (`GameplayStatics.GetPlayerController` 0))
  (if (not (`self.clicked`))
    (set `self.clicked` true)
    (switch `/Game/FirstPerson/Blueprints/Enum/E_Button` (`self.E_Button`)
      (:`NewEnumerator0`
        (`KismetSystemLibrary.QuitGame` (`GameplayStatics.GetPlayerController` 0) "Quit"))
      (:`NewEnumerator1`
        (set `PlayerController.bShowMouseCursor` false _returnvalue)
        (`GameplayStatics.OpenLevel` "Level_Euclidian1")
        (`WidgetBlueprintLibrary.SetInputMode_GameOnly` _returnvalue)))))

(fn `GetInteractiveState`
  (returns (state :type "/Game/FirstPerson/Blueprints/Enum/E_SelectInterface Enum"))
  (return "NewEnumerator1"))

(fn `UserConstructionScript`)