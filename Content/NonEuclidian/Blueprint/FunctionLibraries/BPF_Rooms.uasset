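; Blueprint function library of room and passage helpers, handling passage data records that pair a passage with two platform positions.
; Builds those records from the static mesh components found in sphere-cast hits, using their world locations.
; Lookups find a passage's record in an array or return its opposite endpoint using a tolerance match.
; Smaller helpers convert a string's last character to an integer and gather hit positions, returning inside the loop after the first.
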(fn `FindDataFromLastPassage`
  (params (Passage :type "PrimitiveComponent Object Reference") (DataArray :type "Array of /Game/NonEuclidian/Data/Struct/S_RoomPassages Structure"))
  (returns (Data :type "/Game/NonEuclidian/Data/Struct/S_RoomPassages Structure"))
  (for _array_element DataArray
    (if (== (`.Passage_9_712F06F94E88E76B0C853BA25173C8F6` (break `/Game/NonEuclidian/Data/Struct/S_RoomPassages` _array_element)) Passage)
      (return _array_element))))

(fn `GetLastCharacterInStringAsInt`
  (params (String :type String))
  (returns (Int :type Integer))
  (bind _returnvalue (`KismetStringLibrary.GetCharacterArrayFromString` String))
  (return (`KismetStringLibrary.Conv_StringToInt` (`|GetArrayItem` _returnvalue (`KismetArrayLibrary.Array_LastIndex` _returnvalue)))))

(fn `GetOtherPosFromPassageData`
  (params (PassageData :type "/Game/NonEuclidian/Data/Struct/S_RoomPassages Structure") (Pos :type "Vector Structure"))
  (returns (OtherPos :type "Vector Structure"))
  (bind (_passage _pos1 _pos2) (break `/Game/NonEuclidian/Data/Struct/S_RoomPassages` PassageData))
  (if (== Pos _pos1 :`ErrorTolerance` 1.0)
    (return _pos2)
    (else
      (return _pos1))))

(fn `MakePassageDataFromSphereCastHits`
  (params (Hits :type "Array of HitResult Structure") (Passage :type "PrimitiveComponent Object Reference"))
  (returns (Data :type "/Game/NonEuclidian/Data/Struct/S_RoomPassages Structure"))
  (locals (Platform1 :type "StaticMeshComponent Object Reference") (Platform2 :type "StaticMeshComponent Object Reference"))
  (for _array_element Hits
    (bind _asstatic_mesh_component (cast `StaticMeshComponent` (`.HitComponent` (`GameplayStatics.BreakHitResult` _array_element))))
    (`/Engine/EditorBlueprintResources/StandardMacros.IsValid` (`local.Platform1`)
      (:`Is Valid`
        (set `local.Platform2` _asstatic_mesh_component))
      (:`Is Not Valid`
        (set `local.Platform1` _asstatic_mesh_component))))
  (return (make `/Game/NonEuclidian/Data/Struct/S_RoomPassages` Passage (`SceneComponent.K2_GetComponentLocation` (`local.Platform1`)) (`SceneComponent.K2_GetComponentLocation` (`local.Platform2`)))))

(fn `MakePosArrayFromSphereCastHits`
  (params (Hits :type "Array of HitResult Structure") (TargetArray :type "Array of Vector Structure (by ref)"))
  (returns (Positions :type "Array of Vector Structure"))
  (locals (PosArray :type "Array of Vector Structure"))
  (bind _posarray (`local.PosArray`))
  (for _array_element Hits
    (`KismetArrayLibrary.Array_Add` _posarray (`SceneComponent.K2_GetComponentLocation` (`.HitComponent` (`GameplayStatics.BreakHitResult` _array_element))))
    (return _posarray)))