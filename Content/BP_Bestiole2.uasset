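; BP_Bestiole2 is a wandering creature pawn that stops to face the first-person player when they come close.
; It loops through picking a nearby navigable point, turning toward it, moving via AI MoveTo and pausing randomly.
; A repeating timer, rather than Tick, checks player distance, halting movement and applying yaw-only rotation.
; A flag blocks the wander restart while watching, then relaunches it once the player leaves.
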(event `self.ReceiveBeginPlay`
  (bind _returnvalue (`GameplayStatics.GetActorOfClass` "/Game/FirstPerson/Blueprints/BP_FirstPersonCharacter.BP_FirstPersonCharacter_C"))
  (`/Engine/EditorBlueprintResources/StandardMacros.IsValid` _returnvalue
    (:`Is Valid`
      (set `self.Player` _returnvalue)
      (`KismetSystemLibrary.K2_SetTimerDelegate` (delegate `CE_RotateOnPlayerProximity`) 0.1 true))
    (:`Is Not Valid`
      _))
  (bind _randomlocation (`NavigationSystemV1.K2_GetRandomLocationInNavigableRadius` (`self.K2_GetActorLocation`) 500.0 null null :!label _label))
  (`self.K2_SetActorRotation` (`KismetMathLibrary.FindLookAtRotation` (`self.K2_GetActorLocation`) _randomlocation))
  (`|AIMoveTo` self _randomlocation null
    (:`OnSuccess`
      _)
    (:`OnFail`
      _))
  (`KismetSystemLibrary.Delay` (`KismetMathLibrary.RandomFloatInRange` 1.0 3.0))
  (if (not (or (> (`KismetMathLibrary.VSize` (`self.GetVelocity`)) 10.0) (`self.WasLookingAtPlayerLastFrame`)))
    (`self.CE_StartOver`)))

(event `CE_StartOver`
  (goto _label))

(event `CE_RotateOnPlayerProximity`
  (`/Engine/EditorBlueprintResources/StandardMacros.IsValid` (`self.Player`)
    (:`Is Valid`
      (if (< (`KismetMathLibrary.Vector_Distance` (`self.K2_GetActorLocation`) (`self.K2_GetActorLocation` (`self.Player`))) 300.0)
        (`NavMovementInterface.StopActiveMovement` (`self.FloatingPawnMovement`))
        (`self.K2_SetActorRotation` (`KismetMathLibrary.MakeRotator` 0.0 0.0 (.yaw (`KismetMathLibrary.FindLookAtRotation` (`self.K2_GetActorLocation`) (`self.K2_GetActorLocation` (`self.Player`))))))
        (set `self.WasLookingAtPlayerLastFrame` true)
        (elif (`self.WasLookingAtPlayerLastFrame`)
          (`self.CE_StartOver`)
          (set `self.WasLookingAtPlayerLastFrame` false))))))

(fn `UserConstructionScript`)