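; BP_TunnelCloser is a trigger Blueprint that repositions a referenced object when its Box is overlapped, apparently to close a tunnel.
; With Enter set, the first overlap plays the T_Lift timeline, easing ObjectToLift from its current location, re-read each update, toward ObjectTarget.
; With Enter unset, every overlap instantly moves ObjectToLift to ObjectToBlock's location.
; The overlapping actor is not filtered.
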(event `self.Box.OnComponentBeginOverlap`
  (params (OverlappedComponent :type "PrimitiveComponent Object Reference") (OtherActor :type "Actor Object Reference") (OtherComp :type "PrimitiveComponent Object Reference") (OtherBodyIndex :type Integer) (bFromSweep :type Boolean) (SweepResult :type "HitResult Structure (by ref)"))
  (if (`self.enter`)
    (if (not (`self._hasEntered`))
      ;[0.15 0 0 0.5] Enter Logic
      (set `self._hasEntered` true)
      (set `self._targetV` (`self.K2_GetActorLocation` (`self._objectTarget`)))
      (bind (_direction _alpha) (`Timeline|T_Lift` :!via `PlayFromStart`)
        (:`Update`
          (`self.K2_SetActorLocation` (`self._objectToLift`) (`|EaseFunction` "EaseInOut" _alpha (`self.K2_GetActorLocation` (`self._objectToLift`)) (`self._targetV`)) false false))))
    (else
      (`self.K2_SetActorLocation` (`self._objectToLift`) (`self.K2_GetActorLocation` (`self.ObjectToBlock`)) false false))))

(fn `UserConstructionScript`)