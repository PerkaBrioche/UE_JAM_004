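; BP_Ordi is a computer Blueprint that fades its screen in when the computer boots up.
; On BeginPlay it binds a custom event to the boot-up screen dispatcher on its Ordi reference.
; The first time that event fires, a flag blocks repeats and a timeline drives the screen fade-in multiplier in a Material Parameter Collection.
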(event `self.ReceiveBeginPlay`
  (add `/Game/BP_OrdiButton.ED_BootUpScreen` (`self.Ordi`) (delegate `CE_SetScreenOn`)))

(event `CE_SetScreenOn`
  (if (not (`self.HasBeenSwitchedOn`))
    (set `self.HasBeenSwitchedOn` true)
    (bind (_direction _value) (`Timeline|Timeline` :!via `PlayFromStart`)
      (:`Update`
        _)
      (:`Finished`
        _))
    (`KismetMaterialLibrary.SetScalarParameterValue` (`self.MPC`) "ScreenFadeInCurrentMultiplier" _value)))

(fn `UserConstructionScript`)