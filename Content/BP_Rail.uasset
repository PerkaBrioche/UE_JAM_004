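; Monorail spline actor that carries suspended doors along its track, building the rail from spline meshes in the construction script.
; BeginPlay spawns doors at regular spacing, using non-Euclidean portal doors at chosen indices and linking two as a pair, then starts an initial move.
; Tick advances each door by its stored spline distance, wrapping at the end.
; Two buttons start moves that stop after one or two such wraps.
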(event `self.ReceiveBeginPlay`
  (bind _euclidiandoor1 (`self.EuclidianDoor1`))
  (bind _euclidiandoor2 (`self.EuclidianDoor2`))
  (bind (_returnvalue_location _returnvalue_rotation _returnvalue_scale) (`KismetMathLibrary.BreakTransform` (`SplineComponent.GetTransformAtDistanceAlongSpline` (`self.Spline`) (`self.IncrementalSpacing`) "World" false)))
  (add `/Game/BP_RailButton.ED_StartRailMovement` (`self.ButtonMoveOnce`) (delegate `CE_OnRailStartMovementOnce`))
  (add `/Game/BP_RailButton.ED_StartRailMovement` (`self.ButtonMoveTwice`) (delegate `CE_OnRailStartMovementTwice`))
  (for _index (range (+ (`.ReturnValue` (`KismetMathLibrary.FMod` (`SplineComponent.GetSplineLength` (`self.Spline`)) (`self.DoorSpacing`))) 1))
    (set `self.IncrementalSpacing` (+ (`self.IncrementalSpacing`) (`self.DoorSpacing`)))
    (if (!= (`KismetArrayLibrary.Array_Find` (`self.NonEuclideanDoorsIndices`) _index) -1)
      (set `self.DoorToSpawn` "/Game/BP_EuclidianDoorSuspended.BP_EuclidianDoorSuspended_C")
      (set `self.DoorVerticalOffset` (0.0 0.0 -240.0))
      (else
        (set `self.DoorToSpawn` "/Game/BP_DoorOnRail.BP_DoorOnRail_C")
        (set `self.DoorVerticalOffset` (0.0 0.0 -250.0))))
    (bind _returnvalue (`|SpawnActorFromClass` (`self.DoorToSpawn`) (`KismetMathLibrary.MakeTransform` (+ _returnvalue_location (`self.DoorVerticalOffset`)) (`KismetMathLibrary.ComposeRotators` _returnvalue_rotation (struct :`Yaw` 90.0)) _returnvalue_scale) "Undefined" "MultiplyWithRoot" null null))
    (if (== (`self.DoorToSpawn`) "/Game/BP_EuclidianDoorSuspended.BP_EuclidianDoorSuspended_C")
      (bind _asbp_euclidian_door_suspended (cast `/Game/BP_EuclidianDoorSuspended` _returnvalue))
      (`/Engine/EditorBlueprintResources/StandardMacros.IsValid` (`self.EuclidianDoor1`)
        (:`Is Valid`
          (set `self.EuclidianDoor2` _asbp_euclidian_door_suspended))
        (:`Is Not Valid`
          (set `self.EuclidianDoor1` _asbp_euclidian_door_suspended))))
    (`BlueprintMapLibrary.Map_Add` (`self.SpawnedActors`) _returnvalue (`self.IncrementalSpacing`)))
  (set `/Game/BP_EuclidianDoorSuspended._linkedPortal` (`self.EuclidianDoor2`) (`self.EuclidianDoor1`))
  (set `/Game/BP_EuclidianDoorSuspended._linkedPortal` (`self.EuclidianDoor1`) (`self.EuclidianDoor2`))
  (`/Game/BP_EuclidianDoorSuspended.CE_OnLateSet` _euclidiandoor1)
  (set `/Game/BP_EuclidianDoorSuspended._renderDoor` true _euclidiandoor1)
  (`/Game/BP_EuclidianDoorSuspended.CE_OnLateSet` _euclidiandoor2)
  (set `/Game/BP_EuclidianDoorSuspended._renderDoor` true _euclidiandoor2)
  (`self.CE_StartMovement` false))

(event `CE_OnRailStartMovementOnce`
  (`self.CE_StartMovement` false))

(event `CE_OnRailStartMovementTwice`
  (`self.CE_StartMovement` true))

(event `self.ReceiveTick`
  (params (DeltaSeconds :type "Float (single-precision)"))
  (if (`self.IsMoving`)
    (bind _keys (`BlueprintMapLibrary.Map_Keys` (`self.SpawnedActors`)))
    (for _array_element _keys
      (`self.MoveActor` _array_element (`BlueprintMapLibrary.Map_Find` (`self.SpawnedActors`) _array_element)))))

(event `CE_StartMovement`
  (params (IsMoveTwice :type Boolean))
  (if (not (`self.IsMoving`))
    (if IsMoveTwice
      (set `self.HasMovedOnce` false)
      (else
        (set `self.HasMovedOnce` true)))
    (set `self.IsMoving` true)))

(event `CE_StopMovement`
  (if (`self.HasMovedOnce`)
    (set `self.IsMoving` false)
    (else
      (set `self.HasMovedOnce` true))))

(fn `MoveActor`
  (params (Actor :type "Actor Object Reference") (Distance :type "Float (double-precision)"))
  (locals (`New Distance` :type "Float (double-precision)"))
  (bind (_returnvalue_x _returnvalue_y _returnvalue_z) (`KismetMathLibrary.BreakVector` (`self.K2_GetActorLocation` Actor)))
  (bind (_returnvalue_x_2 _returnvalue_y_2 _returnvalue_z_2) (`KismetMathLibrary.BreakVector` (`SplineComponent.GetLocationAtDistanceAlongSpline` (`self.Spline`) Distance "World")))
  (bind (_returnvalue_location _returnvalue_rotation _returnvalue_scale) (`KismetMathLibrary.BreakTransform` (`SplineComponent.GetTransformAtDistanceAlongSpline` (`self.Spline`) (`local.New Distance`) "World" false)))
  (set `self.DoorVerticalOffset` (`KismetMathLibrary.MakeVector` 0.0 0.0 (- _returnvalue_z _returnvalue_z_2)))
  (bind _output_get (set `local.New Distance` (+ Distance (* (`self.DoorSpeed`) (`GameplayStatics.GetWorldDeltaSeconds`)))))
  (if (>= _output_get (`SplineComponent.GetSplineLength` (`self.Spline`)))
    (set `local.New Distance` 0.0)
    (`self.CE_StopMovement`))
  (`self.K2_SetActorTransform` Actor (`KismetMathLibrary.MakeTransform` (+ _returnvalue_location (`self.DoorVerticalOffset`)) (`KismetMathLibrary.ComposeRotators` _returnvalue_rotation (struct :`Yaw` 90.0)) _returnvalue_scale) false false)
  (`BlueprintMapLibrary.Map_Add` (`self.SpawnedActors`) Actor (`local.New Distance`)))

(fn `UserConstructionScript`
  (for _index (range (`SplineComponent.GetNumberOfSplinePoints` (`self.Spline`)))
    (bind _returnvalue (`AddComponent|NODE_AddSplineMeshComponent-0`))
    (`StaticMeshComponent.SetStaticMesh` _returnvalue "/Game/FirstPerson/Models/MONORAIL_straight.MONORAIL_straight")
    (`PrimitiveComponent.SetCollisionObjectType` _returnvalue "ECC_WorldStatic")
    (`SplineMeshComponent.SetStartRollDegrees` _returnvalue -90.0 true)
    (`SplineMeshComponent.SetEndRollDegrees` _returnvalue -90.0 true)
    (`SplineMeshComponent.SetForwardAxis` _returnvalue "Y" true)
    (bind _returnvalue_2 (+ _index 1))
    (`SplineMeshComponent.SetStartAndEnd` _returnvalue (`SplineComponent.GetLocationAtSplinePoint` (`self.Spline`) _index "Local") (`SplineComponent.GetTangentAtSplinePoint` (`self.Spline`) _index "Local") (`SplineComponent.GetLocationAtSplinePoint` (`self.Spline`) _returnvalue_2 "Local") (`SplineComponent.GetTangentAtSplinePoint` (`self.Spline`) _returnvalue_2 "Local") true)))