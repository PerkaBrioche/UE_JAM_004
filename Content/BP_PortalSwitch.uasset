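; BP_PortalSwitch is a box-triggered switch that changes which portal doors are active when something overlaps it.
; A FlipFlop's first branch calls CESetRender(true) on DoorToActivate entries and, inside that loop, destroys the DoorToDeActivate actors and the switch itself.
; The second branch reverses rendering on both arrays, but runs only if the switch survives the first, as when DoorToActivate is empty.
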(event `self.Box.OnComponentBeginOverlap`
  (params (OverlappedComponent :type "PrimitiveComponent Object Reference") (OtherActor :type "Actor Object Reference") (OtherComp :type "PrimitiveComponent Object Reference") (OtherBodyIndex :type Integer) (bFromSweep :type Boolean) (SweepResult :type "HitResult Structure (by ref)"))
  (`/Engine/EditorBlueprintResources/StandardMacros.FlipFlop`
    (:`A`
      (for _array_element (`self.DoorToActivate`)
        (`/Game/EuclidianDoor.CE_SetRender` _array_element true)
        (for _array_element_2 (`self.DoorToDeActivate`)
          (`self.K2_DestroyActor` _array_element_2))
        (`self.K2_DestroyActor`)))
    (:`B`
      (for _array_element_3 (`self.DoorToActivate`)
        (`/Game/EuclidianDoor.CE_SetRender` _array_element_3 false)
        (for _array_element_4 (`self.DoorToDeActivate`)
          (`/Game/EuclidianDoor.CE_SetRender` _array_element_4 true))))))

(fn `UserConstructionScript`)