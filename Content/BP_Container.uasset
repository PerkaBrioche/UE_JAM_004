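; BP_Container is a container actor with animated double doors and a second pair of doors revealed on demand.
; CE_CloseDoors swings both doors in opposite yaw directions from their BeginPlay rotations via a Timeline, using a scaled, clamped alpha to finish the swing early.
; On completion it sets IsDoorClosed, blocking replays.
; GoodDoor components start hidden; CE_ShowSideDoors makes them visible and collidable after a short delay.
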(event `self.ReceiveBeginPlay`
  (set `self.Rot Right` (.yaw (`SceneComponent.RelativeRotation` (`self.DoorRight`))))
  (set `self.Rot Left` (.yaw (`SceneComponent.RelativeRotation` (`self.DoorLeft`))))
  (`SceneComponent.SetVisibility` (`self.GoodDoorLeft`) false false)
  (`SceneComponent.SetVisibility` (`self.GoodDoorRight`) false false))

(event `CE_CloseDoors`
  (if (not (`self.IsDoorClosed`))
    (bind (_direction _value) (`Timeline|Timeline` :!via `PlayFromStart`)
      (:`Update`
        (bind _returnvalue (`KismetMathLibrary.Lerp` 0.0 130.0 (`KismetMathLibrary.FClamp` (* _value 3.0))))
        (`SceneComponent.K2_SetRelativeRotation` (`self.DoorRight`) (`KismetMathLibrary.MakeRotator` 0.0 0.0 (+ (`self.Rot Right`) _returnvalue)) false false)
        (`SceneComponent.K2_SetRelativeRotation` (`self.DoorLeft`) (`KismetMathLibrary.MakeRotator` 0.0 0.0 (- (`self.Rot Left`) _returnvalue)) false false))
      (:`Finished`
        (set `self.IsDoorClosed` true)))))

(event `CE_ShowSideDoors`
  (bind _gooddoorright (`self.GoodDoorRight`))
  (bind _gooddoorleft (`self.GoodDoorLeft`))
  (`KismetSystemLibrary.Delay` 0.4)
  (`SceneComponent.SetVisibility` _gooddoorleft true false)
  (`PrimitiveComponent.SetCollisionEnabled` _gooddoorleft "QueryAndPhysics")
  (`SceneComponent.SetVisibility` _gooddoorright true false)
  (`PrimitiveComponent.SetCollisionEnabled` _gooddoorright "QueryAndPhysics"))

(fn `UserConstructionScript`)